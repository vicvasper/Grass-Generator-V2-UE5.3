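; Grass instancer actor that scatters a chosen mesh across a landscape as hierarchical instanced static mesh instances.
; SnapToLandscape fits the bounding box to the first Landscape found, and DeleteInstances clears the result.
; GenerateInstances sphere-traces downward over a jittered subdivision grid of the box, optionally keeping only points whose physical material matches CustomLayer.
; Instances take pitch and yaw from the hit normal, with random roll and per-axis scale.
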(fn `0:_SnapToLandscape`
  (bind _returnvalue (`GameplayStatics.GetActorOfClass` "/Script/Landscape.Landscape"))
  (`/Engine/EditorBlueprintResources/StandardMacros.IsValid` _returnvalue
    (:`Is Valid`
      (bind (_origin _boxextent) (`self.GetActorBounds` _returnvalue false false))
      (`BoxComponent.SetBoxExtent` (`self.Bounding Box`) _boxextent true)
      (`self.K2_SetActorLocation` _origin false true))))

(fn `1:_GenerateInstances`
  (bind _subdivisions (`self.Subdivisions`))
  (bind _offset (`self.Offset`))
  (bind _offset_2 (`self.Offset`))
  (bind _returnvalue (`KismetMathLibrary.RandomFloatInRange` (`self.ScaleMin`) (`self.ScaleMax`)))
  (bind (_returnvalue_x _returnvalue_y) (`KismetMathLibrary.BreakVector` (`SceneComponent.K2_GetComponentLocation` (`self.Bounding Box`))))
  (bind _returnvalue_2 (* _subdivisions -1))
  (bind _returnvalue_3 (`GameplayStatics.GetActorOfClass` "/Script/Landscape.Landscape"))
  (`/Engine/EditorBlueprintResources/StandardMacros.IsValid` _returnvalue_3
    (:`Is Valid`
      (`StaticMeshComponent.SetStaticMesh` (`self.HierarchicalInstancedStaticMesh`) (`self.InstancedObject`))
      (bind _output_get (set `self.Extent` (`BoxComponent.BoxExtent` (`self.Bounding Box`))))
      (bind (_returnvalue_x_2 _returnvalue_y_2) (`KismetMathLibrary.BreakVector` (/ _output_get (`self.Subdivisions`))))
      (set `self.DistanceX` _returnvalue_x_2)
      (set `self.DistanceY` _returnvalue_y_2)
      (for _index (range _returnvalue_2 (+ _subdivisions 1))
        (for _index_2 (range _returnvalue_2 (+ _subdivisions 1))
          (bind _returnvalue_4 (+ (+ _returnvalue_x (* (`self.DistanceX`) _index)) (`KismetMathLibrary.RandomFloatInRange` (* _offset_2 -1.0) _offset_2)))
          (bind _returnvalue_5 (+ (+ _returnvalue_y (* (`self.DistanceY`) _index_2)) (`KismetMathLibrary.RandomFloatInRange` (* _offset -1.0) _offset)))
          (bind _outhit (`KismetSystemLibrary.SphereTraceSingleForObjects` :`Start` (`KismetMathLibrary.MakeVector` _returnvalue_4 _returnvalue_5 6000.0) :`End` (`KismetMathLibrary.MakeVector` _returnvalue_4 _returnvalue_5 -400.0) :`Radius` 5.0 :`ObjectTypes` (`|MakeArray` "ObjectTypeQuery1" :!type "EObjectTypeQuery Enum") :`bTraceComplex` true :`DrawTime` 4.0))
          (if (`self.UseCustomLayer`)
            (bind (_bblockinghit _binitialoverlap _time _distance _location _impactpoint _normal _impactnormal _physmat) (`GameplayStatics.BreakHitResult` _outhit))
            (if (== _physmat (`self.CustomLayer`))
              (bind (_returnvalue_roll _returnvalue_pitch _returnvalue_yaw) (`KismetMathLibrary.BreakRotator` (`KismetMathLibrary.Conv_VectorToRotator` _impactnormal)))
              (`InstancedStaticMeshComponent.AddInstance` (`self.HierarchicalInstancedStaticMesh`) (`KismetMathLibrary.MakeTransform` _impactpoint (`KismetMathLibrary.MakeRotator` (`KismetMathLibrary.RandomFloatInRange` (`self.RotationMin`) (`self.RotationMax`)) (- _returnvalue_pitch 90.0) _returnvalue_yaw) (`KismetMathLibrary.MakeVector` _returnvalue _returnvalue _returnvalue)) true :!label _label))
            (else
              (goto _label))))))))

(fn `2:_DeleteInstances`
  (`InstancedStaticMeshComponent.ClearInstances` (`self.HierarchicalInstancedStaticMesh`)))

(fn `UserConstructionScript`)